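; AI trigger volume that waits for the dog (SideScrollerCharacter) and KidCharacterBP, then changes the player's camera and movement.
; Overlap events set presence flags; the child flag stays true after leaving, while the dog flag clears.
; While both are set, Tick raises AIProgress02 and optionally pushes camera rotation, length and offset to the player.
; An optional movement stage either allows forward movement or blocks it and snaps the player's X position.
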(event OnComponentBeginOverlap(CollisionComponent)
  (params (OverlappedComponent :type Primitive%20Component%20Object%20Reference) (OtherActor :type Actor%20Object%20Reference) (OtherComp :type Primitive%20Component%20Object%20Reference) (OtherBodyIndex :type Integer) (bFromSweep :type Boolean) (SweepResult :type Hit%20Result%20Structure%20%28by%20ref%29))
  (Utilities|Casting|CastToSideScrollerCharacter OtherActor
    (:then
      (Variables|Default|SetisDog true))
    (:CastFailed
      _))
  (Utilities|Casting|CastToKidCharacterBP OtherActor)
  (Variables|Default|SetisChild true))

(event OnComponentEndOverlap(CollisionComponent)
  (params (OverlappedComponent :type Primitive%20Component%20Object%20Reference) (OtherActor :type Actor%20Object%20Reference) (OtherComp :type Primitive%20Component%20Object%20Reference) (OtherBodyIndex :type Integer))
  (Utilities|Casting|CastToSideScrollerCharacter OtherActor
    (:then
      (Variables|Default|SetisDog false))
    (:CastFailed
      _))
  (Utilities|Casting|CastToKidCharacterBP OtherActor)
  (Variables|Default|SetisChild true))

(event EventBeginPlay)

(event EventTick
  (params (DeltaSeconds :type Float%20%28single-precision%29))
  (if (Variables|Default|GetisDog)
    (if (Variables|Default|GetisChild)
      (Variables|Default|SetAI_Progress02 true)
      (if (Variables|Default|GetCamera)
        ;[1 1 1] Camera
        (bind _asside_scroller_character (Utilities|Casting|CastToSideScrollerCharacter (Game|GetPlayerCharacter 0)))
        (Variables|/Game/SideScrollerCPP/Blueprints/SideScrollerCharacter.SideScrollerCharacter_C|SetCamera%20Switch _asside_scroller_character true)
        (Variables|/Game/SideScrollerCPP/Blueprints/SideScrollerCharacter.SideScrollerCharacter_C|SetCamera%20Rot _asside_scroller_character (Variables|Default|GetTrigger_Rot))
        (Variables|/Game/SideScrollerCPP/Blueprints/SideScrollerCharacter.SideScrollerCharacter_C|SetCamera%20Length _asside_scroller_character (Variables|Default|GetTrigger_Legnth))
        (Variables|/Game/SideScrollerCPP/Blueprints/SideScrollerCharacter.SideScrollerCharacter_C|SetCamera%20Offset _asside_scroller_character (Variables|Default|GetTrigger_Offset)))
      (if (Variables|Default|GetMovement)
        ;[1 1 1] Movement
        (bind _asside_scroller_character_2 (Utilities|Casting|CastToSideScrollerCharacter (Game|GetPlayerCharacter 0)))
        (if (Variables|Default|GetLockMovement)
          (Variables|/Script/SideScroller.SideScrollerCharacter|SetMoveForwards _asside_scroller_character_2 false)
          (Transformation|SetActorLocation _asside_scroller_character_2 (Math|Vector|Lerp(Vector) (Math|Vector|MakeVector (.x (Transformation|GetActorLocation _asside_scroller_character_2)) (.y (Transformation|GetActorLocation _asside_scroller_character_2)) (.z (Transformation|GetActorLocation _asside_scroller_character_2))) (Math|Vector|MakeVector (.x (Variables|Default|GetNewActorLocation)) (.y (Transformation|GetActorLocation _asside_scroller_character_2)) (.z (Transformation|GetActorLocation _asside_scroller_character_2))) 1.0) false false)
          (else
            (Variables|/Script/SideScroller.SideScrollerCharacter|SetMoveForwards _asside_scroller_character_2 true)))))))

(fn ConstructionScript)