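; A pushable cube actor for a side-scroller that the player character can move.
; X-axis and Y-axis collision components enable player input on the cube when an overlap begins and disable it when one ends.
; For a SideScrollerCharacter, overlaps also toggle the character's IsPushing flag.
; Cube physics simulation is switched on at both begin and end overlap and is never switched off here.
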(event OnComponentBeginOverlap(Y-axisCollision)
  (params (OverlappedComponent :type Primitive%20Component%20Object%20Reference) (OtherActor :type Actor%20Object%20Reference) (OtherComp :type Primitive%20Component%20Object%20Reference) (OtherBodyIndex :type Integer) (bFromSweep :type Boolean) (SweepResult :type Hit%20Result%20Structure%20%28by%20ref%29))
  ;[1 1 1] Y-Axis Collision
  (Input|EnableInput (Game|GetPlayerController 0))
  (bind _asside_scroller_character (Utilities|Casting|CastToSideScrollerCharacter OtherActor))
  (Physics|SetSimulatePhysics (Variables|Default|GetCube) true)
  (Variables|/Script/SideScroller.SideScrollerCharacter|SetIsPushing _asside_scroller_character true))

(event OnComponentBeginOverlap(X-axisCollision)
  (params (OverlappedComponent :type Primitive%20Component%20Object%20Reference) (OtherActor :type Actor%20Object%20Reference) (OtherComp :type Primitive%20Component%20Object%20Reference) (OtherBodyIndex :type Integer) (bFromSweep :type Boolean) (SweepResult :type Hit%20Result%20Structure%20%28by%20ref%29))
  ;[1 1 1] X-Axis Collision
  (Input|EnableInput (Game|GetPlayerController 0))
  (bind _asside_scroller_character (Utilities|Casting|CastToSideScrollerCharacter OtherActor))
  (Physics|SetSimulatePhysics (Variables|Default|GetCube) true)
  (Variables|/Script/SideScroller.SideScrollerCharacter|SetIsPushing _asside_scroller_character true))

(event OnComponentEndOverlap(X-axisCollision)
  (params (OverlappedComponent :type Primitive%20Component%20Object%20Reference) (OtherActor :type Actor%20Object%20Reference) (OtherComp :type Primitive%20Component%20Object%20Reference) (OtherBodyIndex :type Integer))
  ;[1 1 1] X-Axis Collision
  (Input|DisableInput (Game|GetPlayerController 0))
  (bind _asside_scroller_character (Utilities|Casting|CastToSideScrollerCharacter OtherActor))
  (Physics|SetSimulatePhysics (Variables|Default|GetCube) true)
  (Variables|/Script/SideScroller.SideScrollerCharacter|SetIsPushing _asside_scroller_character false))

(event OnComponentEndOverlap(Y-axisCollision)
  (params (OverlappedComponent :type Primitive%20Component%20Object%20Reference) (OtherActor :type Actor%20Object%20Reference) (OtherComp :type Primitive%20Component%20Object%20Reference) (OtherBodyIndex :type Integer))
  ;[1 1 1] Y-Axis Collision
  (Input|DisableInput (Game|GetPlayerController 0))
  (bind _asside_scroller_character (Utilities|Casting|CastToSideScrollerCharacter OtherActor))
  (Physics|SetSimulatePhysics (Variables|Default|GetCube) true)
  (Variables|/Script/SideScroller.SideScrollerCharacter|SetIsPushing _asside_scroller_character false))

(fn ConstructionScript)