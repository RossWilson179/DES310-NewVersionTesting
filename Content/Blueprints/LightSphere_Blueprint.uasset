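; Light sphere actor that glows blue while the side-scroller character stands inside its box trigger.
; Box overlap events swap the mesh between lit and dark materials and toggle the point light, with the LightsOut flag blocking activation on entry.
; Off forces the dark state, while On relights the sphere only if the player character is already overlapping the box.
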(event OnComponentBeginOverlap(Box)
  (params (OverlappedComponent :type Primitive%20Component%20Object%20Reference) (OtherActor :type Actor%20Object%20Reference) (OtherComp :type Primitive%20Component%20Object%20Reference) (OtherBodyIndex :type Integer) (bFromSweep :type Boolean) (SweepResult :type Hit%20Result%20Structure%20%28by%20ref%29))
  (if (not (Variables|Default|GetLightsOut))
    (Utilities|Casting|CastToSideScrollerCharacter OtherActor)
    (Rendering|Material|SetMaterial (Variables|Debug|GetStaticMeshComponent self) 0 "/Game/Materials/TestMaterials/BlueLightTest.BlueLightTest")
    (Rendering|SetVisibility (Variables|Default|GetPointLight) true false)))

(event OnComponentEndOverlap(Box)
  (params (OverlappedComponent :type Primitive%20Component%20Object%20Reference) (OtherActor :type Actor%20Object%20Reference) (OtherComp :type Primitive%20Component%20Object%20Reference) (OtherBodyIndex :type Integer))
  (Utilities|Casting|CastToSideScrollerCharacter OtherActor)
  (Rendering|Material|SetMaterial (Variables|Debug|GetStaticMeshComponent self) 0 "/Game/Materials/TestMaterials/Dark.Dark")
  (Rendering|SetVisibility (Variables|Default|GetPointLight) false false))

(event EventBeginPlay)

(event Collision|EventActorBeginOverlap
  (params (OtherActor :type Actor%20Object%20Reference)))

(event EventTick
  (params (DeltaSeconds :type Float%20%28single-precision%29)))

(fn ConstructionScript)

(fn Off
  (Rendering|Material|SetMaterial (Variables|Debug|GetStaticMeshComponent self) 0 "/Game/Materials/TestMaterials/Dark.Dark")
  (Rendering|SetVisibility (Variables|Default|GetPointLight) false false))

(fn On
  (bind _asside_scroller_character (Utilities|Casting|CastToSideScrollerCharacter (Game|GetPlayerCharacter 0)))
  (if (Collision|IsOverlappingActor (Variables|Default|GetBox) _asside_scroller_character :!class /Script/Engine.PrimitiveComponent)
    (Rendering|Material|SetMaterial (Variables|Debug|GetStaticMeshComponent self) 0 "/Game/Materials/TestMaterials/BlueLightTest.BlueLightTest")
    (Rendering|SetVisibility (Variables|Default|GetPointLight) true false)))